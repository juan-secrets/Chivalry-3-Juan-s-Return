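; BP_Archer is a ranged enemy that shoots arrows at the player it perceives.
; AI perception stores a sensed player as the target and starts a looping fire timer; losing it, or any non-player update, clears both.
; Each shot spawns a BP_Arrow at the spawn point, rotated toward the player's capsule.
; The world-space aim direction, scaled to a fixed speed, is passed to the projectile's local-space velocity setter.
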(event OnTargetPerceptionUpdated(AIPerception)
  (params (Actor :type Actor%20Object%20Reference) (Stimulus :type AI%20Stimulus%20Structure))
  (bind _asbp_player (Utilities|Casting|CastToBP_Player Actor)
    (:then
      (if (.bsuccessfullysensed Stimulus)
        (Variables|Default|SetTargetPlayer _asbp_player)
        (Utilities|Time|SetTimerbyFunctionName 0 "Fire Arrow" 3.0 true)
        (Development|PrintString "FOUND")
        (else
          (Variables|Default|SetTargetPlayer 0 :!label _label)
          (Utilities|Time|ClearTimerbyFunctionName 0 "Fire Arrow")
          (Development|PrintString "LOST"))))
    (:CastFailed
      (goto _label))))

(event Custom|Fire%20Arrow
  (bind _targetplayer (Variables|Default|GetTargetPlayer))
  (bind _arrowspawnpoint (Variables|Default|GetArrowSpawnPoint))
  (bind _returnvalue (Transformation|GetWorldLocation _arrowspawnpoint))
  (bind _capsulecomponent (Variables|/Script/Engine.Character|GetCapsuleComponent _targetplayer))
  (bind _returnvalue_2 (Transformation|GetWorldLocation _capsulecomponent))
  (bind _returnvalue_3 (- _returnvalue_2 _returnvalue))
  (bind _returnvalue_4 (Math|Vector|Normalize _returnvalue_3))
  (bind _returnvalue_5 (Math|Rotator|MakeRotfromX _returnvalue_4))
  (Utilities|IsValid (Variables|Default|GetTargetPlayer)
    (:Is%20Valid
      (if true
        (bind _returnvalue_6 (Game|SpawnActorfromClass "/Game/GameAssets/Blueprints/Actor/BP_Arrow.BP_Arrow_C" (Math|Transform|MakeTransform (Transformation|GetWorldLocation (Variables|Default|GetArrowSpawnPoint)) _returnvalue_5 "1.000000,1.000000,1.000000") "AlwaysSpawn" "MultiplyWithRoot" 0 0))
        (bind _output_get (Variables|Default|SetSpawnedArrow _returnvalue_6))
        (Game|Components|ProjectileMovement|SetVelocityinLocalSpace (Variables|/Game/GameAssets/Blueprints/Actor/BP_Arrow.BP_Arrow_C|GetProjectileMovement _output_get) (* (Math|Vector|GetForwardVector _returnvalue_5) 2e+03))
        (Development|PrintString "FIRE" true true "(R=1.000000,G=0.087611,B=0.000000,A=1.000000)")))))

(fn ConstructionScript)