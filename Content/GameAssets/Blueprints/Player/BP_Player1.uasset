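; Player character with directional sword combat, interpolated sprint speed and FOV, NPC dialog interaction, HUD and menu widgets.
; Last look direction selects attack and block animations; frontal hits are parried only when directions match, with left/right mirrored.
; Sword overlap sends damage messages, while per-tick sphere traces between previous and current socket positions place blood effects.
; Tick also drives footstep audio and death, which triggers ragdoll and a dialog.
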(event Input|EnhancedActionEvents|EnhancedInputActionIA_SwitchArrowsDisplay
  (params (ActionValue :type Boolean) (ElapsedSeconds :type Float%20%28double-precision%29) (TriggeredSeconds :type Float%20%28double-precision%29) (InputAction :type Input%20Action%20Object%20Reference :default "/Game/GameAssets/Blueprints/Inputs/IA_SwitchArrowsDisplay.IA_SwitchArrowsDisplay"))
  ;[0.15 0.15 0.15 0.5] Switch Direction Arrow Display
  (:Started
    (if (Variables|Default|GetArrowsEnabled)
      (Variables|Default|SetArrowsEnabled false)
      (Widget|RemovefromParent (Variables|Default|GetDirectionArrows))
      (Variables|Default|SetDirectionArrows 0)
      (else
        (Variables|Default|SetArrowsEnabled true)
        (bind _returnvalue (UserInterface|CreateWidget "/Game/GameAssets/Blueprints/Player/UI/WBP_ActionDirection.WBP_ActionDirection_C"))
        (bind _output_get (Variables|Default|SetDirectionArrows _returnvalue))
        (UserInterface|Viewport|AddtoViewport _output_get 0)))))

(event Input|EnhancedActionEvents|EnhancedInputActionIA_OpenCloseInGameMenu
  (params (ActionValue :type Boolean) (ElapsedSeconds :type Float%20%28double-precision%29) (TriggeredSeconds :type Float%20%28double-precision%29) (InputAction :type Input%20Action%20Object%20Reference :default "/Game/GameAssets/Blueprints/Inputs/IA_OpenCloseInGameMenu.IA_OpenCloseInGameMenu"))
  (bind _returnvalue (Game|GetPlayerController 0))
  ;[0.15 0.15 0.15 0.5] Open/Close In Game Menu
  (UserInterface|Viewport|AddtoViewport (CallFunction|GetinGameMenu) 0)
  (Input|SetInputModeUIOnly _returnvalue (Variables|Default|GetWBP_InGameMenu) "DoNotLock" true)
  (Variables|/Script/Engine.PlayerController|SetbShowMouseCursor _returnvalue true))

(event EventBeginPlay
  ;[0.15 0.15 0.15 0.5] Setup IMC
  (Utilities|FlowControl|DelayUntilNextTick)
  (Input|AddMappingContext (PlayerController|LocalPlayerSubsystems|GetEnhancedInputLocalPlayerSubsystem (Game|GetPlayerController 0)) "/Game/GameAssets/Blueprints/Inputs/IMC_Player.IMC_Player" 0 "(bIgnoreAllPressedKeysUntilRelease=True,bForceImmediately=False,bNotifyUserSettings=False)")
  ;[0.15 0.15 0.15 0.5] Switch Skeletal Mesh Ownership
  (for _array_element (Utilities|Array|MakeArray (Variables|Default|GetSKM_Grian01_Leg_1) (Variables|Default|GetSKM_Grian01_Head_1) (Variables|Default|GetSKM_Grian01_Foot_1) (Variables|Default|GetSKM_Grian01_Hand_1) (Variables|Default|GetSKM_Grian01_Chest_1))
    (Components|SkinnedMesh|SetLeaderPoseComponent _array_element (Variables|Character|GetMesh) false false))
  ;[0.15 0.15 0.15 0.5] Create Health Bar Widget
  (bind _returnvalue (UserInterface|CreateWidget "/Game/GameAssets/Blueprints/Player/UI/WBP_HealthBar.WBP_HealthBar_C"))
  (UserInterface|Viewport|AddtoViewport _returnvalue 0)
  ;[0.15 0.15 0.15 0.5] Create Arrow Direction Widget
  (if (Variables|Default|GetArrowsEnabled)
    (bind _returnvalue_2 (UserInterface|CreateWidget "/Game/GameAssets/Blueprints/Player/UI/WBP_ActionDirection.WBP_ActionDirection_C"))
    (bind _output_get (Variables|Default|SetDirectionArrows _returnvalue_2))
    (UserInterface|Viewport|AddtoViewport _output_get 0)
    ;[0.15 0.15 0.15 0.5] Set Sword Sockets
    (Variables|Default|SetSwordSockets (Transformation|GetAllSocketNames (Variables|Default|GetSM_Sword_001_01)))
    (CallFunction|SetSwordSocketsPosition)
    ;[0.15 0.15 0.15 0.5] Quest Log Widget
    (bind _returnvalue_3 (UserInterface|CreateWidget "/Game/GameAssets/Blueprints/Player/UI/WBP_QuestLog.WBP_QuestLog_C"))
    (UserInterface|Viewport|AddtoViewport _returnvalue_3 0)
    ;[0.15 0.15 0.15 0.5] Set Wlaking Audio Component
    (bind _returnvalue_4 (Audio|CreateSound2D "/Game/GameAssets/Assets/SFX/Characters/FootSteps/SC_FootSteps.SC_FootSteps" 1.0 1.0 0.0 0 true false))
    (Variables|Default|SetWalkingSFX _returnvalue_4)))

(event EventTick
  (params (DeltaSeconds :type Float%20%28single-precision%29))
  (bind _returnvalue (Game|GetPlayerController 0))
  (bind _charactermovement (Variables|Character|GetCharacterMovement))
  (bind _camera (Variables|Default|GetCamera))
  (bind _charactermovement_2 (Variables|Character|GetCharacterMovement))
  (bind _walkingsfx (Variables|Default|GetWalkingSFX))
  (bind _returnvalue_2 (Audio|Components|Audio|IsPlaying _walkingsfx))
  (bind _returnvalue_3 (Pawn|Components|CharacterMovement|GetCurrentAcceleration _charactermovement))
  ;[0.15 0.15 0.15 0.5] Event tick
  (Utilities|FlowControl|Sequence
    (:then_0
      ;[0.15 0.15 0.15 0.5] Update Speed and Camera FOV
      (Variables|/Script/Engine.CharacterMovementComponent|SetMaxWalkSpeed _charactermovement_2 (Math|Interpolation|FInterpTo (Variables|/Script/Engine.CharacterMovementComponent|GetMaxWalkSpeed _charactermovement_2) (Variables|Default|GetTargetSpeed) DeltaSeconds 5.0))
      (Camera|SetFieldOfView _camera (Math|Interpolation|FInterpTo (Variables|/Script/Engine.CameraComponent|GetFieldOfView _camera) (Variables|Default|GetTargetFOV) DeltaSeconds 1e+01)))
    (:then_1
      ;[0.15 0.15 0.15 0.5] Death on Health <= 0
      (if (and (not (Variables|Default|GetisDead)) (<= (Variables|Default|GetHealth) 0))
        (Variables|Default|SetisDead true)
        ;;[0.15 0.15 0.15 0.5] Play Death Sounds
        (Audio|PlaySound2D "/Game/GameAssets/Assets/SFX/Characters/SW_MaleDeathSound.SW_MaleDeathSound" 1.0 1.0 0.0 0 0)
        (Audio|PlaySound2D "/Game/GameAssets/Assets/SFX/Characters/SW_BodyFallImpact.SW_BodyFallImpact" 1.0 1.0 0.0 0 0 false)
        (Utilities|FlowControl|Delay 0.3)
        (Audio|PlaySound2D "/Game/GameAssets/Assets/SFX/Characters/Weapons/SW_SwordFallImpact.SW_SwordFallImpact" 1.0 1.0 0.0 0 0)
        (CallFunction|GoRagdoll)
        (Utilities|FlowControl|Delay 1.0)
        (bind _returnvalue_4 (UserInterface|CreateWidget "/Game/GameAssets/Blueprints/Player/UI/WBP_DeathDialog.WBP_DeathDialog_C"))
        (UserInterface|Viewport|AddtoViewport _returnvalue_4 0)
        (Input|SetInputModeUIOnly _returnvalue _returnvalue_4 "DoNotLock" false)
        (Variables|/Script/Engine.PlayerController|SetbShowMouseCursor _returnvalue true)))
    (:then_2
      ;[0.15 0.15 0.15 0.5] Calculate sword collisions based on sword sockets
      (if (and (Variables|Default|GetisAttacking) (not (Variables|Default|GetAttackInput)))
        (for (_array_element _array_index) (Variables|Default|GetSwordSockets)
          (bind (_outhit _returnvalue_5) (Collision|SphereTraceByChannel (Utilities|Array|Get(acopy) (Variables|Default|GetSwordOldSocketsPositions) _array_index) (Transformation|GetSocketLocation (Variables|Default|GetSM_Sword_001_01) _array_element) 1.0 "TraceTypeQuery2" true 0 "None"))
          (if _returnvalue_5 ; True If Hit occured
            (if (Utilities|DoesObjectImplementInterface (.hitactor _outhit) "/Game/GameAssets/Blueprints/Interfaces/BPI_Fighters.BPI_Fighters_C")
              (CallFunction|AttachBloodParticlestoBone (.hitactor _outhit) (.location _outhit) (.normal _outhit) (.hitbonename _outhit))
              (else
                (CallFunction|SetSwordSocketsPosition :!label _label)))
            (else
              (goto _label))))))
    (:then_3
      ;[0.15 0.15 0.15 0.5] Walking SFX
      (Utilities|FlowControl|DelayUntilNextTick)
      (Utilities|IsValid _walkingsfx
        (:Is%20Valid
          (if (!= (+ (.x _returnvalue_3) (.y _returnvalue_3)) 0.0)
            (if (not _returnvalue_2)
              (Audio|Components|Audio|Play _walkingsfx 0.0))
            (elif _returnvalue_2
              (Audio|Components|Audio|Stop _walkingsfx))))))))

(event Input|EnhancedActionEvents|EnhancedInputActionIA_PlayerMove
  (params (ActionValue :type Vector%202D%20Structure) (ElapsedSeconds :type Float%20%28double-precision%29) (TriggeredSeconds :type Float%20%28double-precision%29) (InputAction :type Input%20Action%20Object%20Reference :default "/Game/GameAssets/Blueprints/Inputs/IA_PlayerMove.IA_PlayerMove"))
  (bind _returnvalue (Pawn|GetControlRotation :!class /Script/Engine.Pawn))
  ;[0.15 0.15 0.15 0.5] Player Move
  (Pawn|Input|AddMovementInput (Math|Vector|GetRightVector (Math|Rotator|MakeRotator 0.0 0.0 (.yaw _returnvalue))) (.x ActionValue) false)
  (Pawn|Input|AddMovementInput (Math|Vector|GetForwardVector (Math|Rotator|MakeRotator 0.0 0.0 (.yaw _returnvalue))) (.y ActionValue) false))

(event Input|EnhancedActionEvents|EnhancedInputActionIA_PlayerJump
  (params (ActionValue :type Boolean) (ElapsedSeconds :type Float%20%28double-precision%29) (TriggeredSeconds :type Float%20%28double-precision%29) (InputAction :type Input%20Action%20Object%20Reference :default "/Game/GameAssets/Blueprints/Inputs/IA_PlayerJump.IA_PlayerJump"))
  ;[0.15 0.15 0.15 0.5] Player Jump
  (:Started
    (Character|Jump))
  (:Completed
    (Character|StopJumping)))

(event Input|EnhancedActionEvents|EnhancedInputActionIA_PlayerLook
  (params (ActionValue :type Vector%202D%20Structure) (ElapsedSeconds :type Float%20%28double-precision%29) (TriggeredSeconds :type Float%20%28double-precision%29) (InputAction :type Input%20Action%20Object%20Reference :default "/Game/GameAssets/Blueprints/Inputs/IA_PlayerLook.IA_PlayerLook"))
  ;[0.15 0.15 0.15 0.5] Player Look
  (Utilities|FlowControl|Sequence
    (:then_0
      (Pawn|Input|AddControllerYawInput (.x ActionValue))
      (Pawn|Input|AddControllerPitchInput (.y ActionValue)))
    (:then_1
      (if (>= (Math|Float|Absolute(Float) (.x ActionValue)) (Math|Float|Absolute(Float) (.y ActionValue))) ; True is Left/Right Look\nFalse is Top/Bottom Look
        (if (>= (.x ActionValue) 0.0) ; True is Right Look\nFalse is Left Look
          (Variables|Default|SetLastLookDirection (Class|KismetMathLibrary|VectorRight))
          (else
            (Variables|Default|SetLastLookDirection (Class|KismetMathLibrary|VectorLeft))))
        (elif (>= 0.0 (.y ActionValue)) ; True is Top Look\nFalse is Bottom Look
          (Variables|Default|SetLastLookDirection (Math|Vector|VectorUp))
          (else
            (Variables|Default|SetLastLookDirection (Math|Vector|VectorDown))))))))

(event Input|EnhancedActionEvents|EnhancedInputActionIA_PlayerSprint
  (params (ActionValue :type Boolean) (ElapsedSeconds :type Float%20%28double-precision%29) (TriggeredSeconds :type Float%20%28double-precision%29) (InputAction :type Input%20Action%20Object%20Reference :default "/Game/GameAssets/Blueprints/Inputs/IA_PlayerSprint.IA_PlayerSprint"))
  ;[0.15 0.15 0.15 0.5] Player Sprint
  (:Started
    (Variables|Default|SetisSprinting true)
    (CallFunction|UpdateSpeedandFOV :!label _label))
  (:Completed
    (Variables|Default|SetisSprinting false)
    (goto _label)))

(event Input|EnhancedActionEvents|EnhancedInputActionIA_PlayerInteract
  (params (ActionValue :type Boolean) (ElapsedSeconds :type Float%20%28double-precision%29) (TriggeredSeconds :type Float%20%28double-precision%29) (InputAction :type Input%20Action%20Object%20Reference :default "/Game/GameAssets/Blueprints/Inputs/IA_PlayerInteract.IA_PlayerInteract"))
  (:Started
    (Utilities|FlowControl|Sequence
      (:then_0
        (for _array_element (Collision|GetOverlappingActors "/Game/GameAssets/Blueprints/AI/BP_Villager.BP_Villager_C" :!class /Script/Engine.Actor)
          (if (Utilities|DoesObjectImplementInterface _array_element "/Game/GameAssets/Blueprints/Dialogs/BPI_Dialog.BPI_Dialog_C")
            (Class|BPIDialog|Talk(Message) _array_element))))
      (:then_1
        (for _array_element_2 (Collision|GetOverlappingActors "/Game/GameAssets/Blueprints/AI/BP_TutorialGuy.BP_TutorialGuy_C" :!class /Script/Engine.Actor)
          (if (Utilities|DoesObjectImplementInterface _array_element_2 "/Game/GameAssets/Blueprints/Dialogs/BPI_Dialog.BPI_Dialog_C")
            (Class|BPIDialog|TutorialTalk(Message) _array_element_2))))
      (:then_2
        (for _array_element_3 (Collision|GetOverlappingActors "/Game/GameAssets/Blueprints/AI/BP_OldMan.BP_OldMan_C" :!class /Script/Engine.Actor)
          (if (Utilities|DoesObjectImplementInterface _array_element_3 "/Game/GameAssets/Blueprints/Dialogs/BPI_Dialog.BPI_Dialog_C")
            (Class|BPIDialog|OldManTalk(Message) _array_element_3 (Variables|Default|GetProgressionIndex))))))))

(event OnComponentBeginOverlap(SM_Sword_001_01)
  (params (OverlappedComponent :type Primitive%20Component%20Object%20Reference) (OtherActor :type Actor%20Object%20Reference) (OtherComp :type Primitive%20Component%20Object%20Reference) (OtherBodyIndex :type Integer) (bFromSweep :type Boolean) (SweepResult :type Hit%20Result%20Structure%20%28by%20ref%29))
  ;[0.15 0.15 0.15 0.5] Hit Player
  (if (and (Class|KismetMathLibrary|XORBoolean (Variables|Default|GetisAttacking) (Variables|Default|GetAttackInput)) (!= OtherActor self))
    (Class|BPIFighters|AttemptHit(Message) OtherActor self (Variables|Default|GetActionDirection) 15)))

(event Input|EnhancedActionEvents|EnhancedInputActionIA_PlayerAttack
  (params (ActionValue :type Boolean) (ElapsedSeconds :type Float%20%28double-precision%29) (TriggeredSeconds :type Float%20%28double-precision%29) (InputAction :type Input%20Action%20Object%20Reference :default "/Game/GameAssets/Blueprints/Inputs/IA_PlayerAttack.IA_PlayerAttack"))
  ;[0.15 0.15 0.15 0.5] Handle Attack
  (:Started
    (if (not (Variables|Default|GetisBlocking))
      (Variables|Default|SetAttackInput true)
      (if (not (Variables|Default|GetisAttacking))
        (Utilities|FlowControl|Sequence
          (:then_0
            (if (Utilities|Operators|EqualEqual (Variables|Default|GetLastLookDirection) (Class|KismetMathLibrary|VectorRight) 0.0)
              (Variables|Default|SetSwordChargeAnim "/Game/GameAssets/Assets/Animations/Sword/Charge/AM_R_SwordCharge.AM_R_SwordCharge")
              (Variables|Default|SetSwordSlashAnim "/Game/GameAssets/Assets/Animations/Sword/Slash/AM_R_SwordSlash.AM_R_SwordSlash")
              (Variables|Default|SetActionDirection (Class|KismetMathLibrary|VectorRight))
              (Variables|Default|SetisAttacking true :!label _label)
              (Utilities|FlowControl|Delay 0.5)
              (Audio|PlaySound2D "/Game/GameAssets/Assets/SFX/Characters/Weapons/SW_SwordSwing.SW_SwordSwing" 1.0 1.0 0.0 0 0)))
          (:then_1
            (if (Utilities|Operators|EqualEqual (Variables|Default|GetLastLookDirection) (Class|KismetMathLibrary|VectorLeft) 0.0)
              (Variables|Default|SetSwordChargeAnim "/Game/GameAssets/Assets/Animations/Sword/Charge/AM_L_SwordCharge.AM_L_SwordCharge")
              (Variables|Default|SetSwordSlashAnim "/Game/GameAssets/Assets/Animations/Sword/Slash/AM_L_SwordSlash.AM_L_SwordSlash")
              (Variables|Default|SetActionDirection (Class|KismetMathLibrary|VectorLeft))
              (goto _label)))
          (:then_2
            (if (Utilities|Operators|EqualEqual (Variables|Default|GetLastLookDirection) (Math|Vector|VectorUp) 0.0)
              (Variables|Default|SetSwordChargeAnim "/Game/GameAssets/Assets/Animations/Sword/Charge/AM_T_SwordCharge.AM_T_SwordCharge")
              (Variables|Default|SetSwordSlashAnim "/Game/GameAssets/Assets/Animations/Sword/Slash/AM_T_SwordSlash.AM_T_SwordSlash")
              (Variables|Default|SetActionDirection (Math|Vector|VectorUp))
              (goto _label)))
          (:then_3
            (if (Utilities|Operators|EqualEqual (Variables|Default|GetLastLookDirection) (Math|Vector|VectorDown) 0.0)
              (Variables|Default|SetSwordChargeAnim "/Game/GameAssets/Assets/Animations/Sword/Charge/AM_B_SwordCharge.AM_B_SwordCharge")
              (Variables|Default|SetSwordSlashAnim "/Game/GameAssets/Assets/Animations/Sword/Slash/AM_B_SwordSlash.AM_B_SwordSlash")
              (Variables|Default|SetActionDirection (Math|Vector|VectorDown))
              (goto _label)))))))
  (:Completed
    (Variables|Default|SetAttackInput false)
    (Utilities|FlowControl|Delay (+ (Math|Float|Clamp(Float) (- (Variables|/Script/Engine.AnimSequenceBase|GetSequenceLength (Variables|Default|GetSwordChargeAnim)) ElapsedSeconds) 0.0 (Variables|/Script/Engine.AnimSequenceBase|GetSequenceLength (Variables|Default|GetSwordChargeAnim))) (Variables|/Script/Engine.AnimSequenceBase|GetSequenceLength (Variables|Default|GetSwordSlashAnim))))
    (Variables|Default|SetisAttacking false)))

(event Input|EnhancedActionEvents|EnhancedInputActionIA_PlayerBlock
  (params (ActionValue :type Boolean) (ElapsedSeconds :type Float%20%28double-precision%29) (TriggeredSeconds :type Float%20%28double-precision%29) (InputAction :type Input%20Action%20Object%20Reference :default "/Game/GameAssets/Blueprints/Inputs/IA_PlayerBlock.IA_PlayerBlock"))
  ;[0.15 0.15 0.15 0.5] Handle Block
  (:Started
    (if (not (Variables|Default|GetisAttacking))
      (Variables|Default|SetBlockInput true)
      (if (not (Variables|Default|GetisBlocking))
        (Utilities|FlowControl|Sequence
          (:then_0
            (if (Utilities|Operators|EqualEqual (Variables|Default|GetLastLookDirection) (Class|KismetMathLibrary|VectorRight) 0.0)
              (Variables|Default|SetBlockAnim "/Game/GameAssets/Assets/Animations/Sword/Block/AM_R_SwordBlock.AM_R_SwordBlock")
              (Variables|Default|SetActionDirection (Class|KismetMathLibrary|VectorRight))
              (Variables|Default|SetisBlocking true :!label _label)))
          (:then_1
            (if (Utilities|Operators|EqualEqual (Variables|Default|GetLastLookDirection) (Class|KismetMathLibrary|VectorLeft) 0.0)
              (Variables|Default|SetBlockAnim "/Game/GameAssets/Assets/Animations/Sword/Block/AM_L_SwordBlock.AM_L_SwordBlock")
              (Variables|Default|SetActionDirection (Class|KismetMathLibrary|VectorLeft))
              (goto _label)))
          (:then_2
            (if (Utilities|Operators|EqualEqual (Variables|Default|GetLastLookDirection) (Math|Vector|VectorUp) 0.0)
              (Variables|Default|SetBlockAnim "/Game/GameAssets/Assets/Animations/Sword/Block/AM_T_SwordBlock.AM_T_SwordBlock")
              (Variables|Default|SetActionDirection (Math|Vector|VectorUp))
              (goto _label)))
          (:then_3
            (if (Utilities|Operators|EqualEqual (Variables|Default|GetLastLookDirection) (Math|Vector|VectorDown) 0.0)
              (Variables|Default|SetBlockAnim "/Game/GameAssets/Assets/Animations/Sword/Block/AM_B_SwordBlock.AM_B_SwordBlock")
              (Variables|Default|SetActionDirection (Math|Vector|VectorDown))
              (goto _label)))))))
  (:Completed
    (Variables|Default|SetBlockInput false)
    (Utilities|FlowControl|Delay (Math|Float|Clamp(Float) (- (Variables|/Script/Engine.AnimSequenceBase|GetSequenceLength (Variables|Default|GetBlockAnim)) ElapsedSeconds) 0.0 (Variables|/Script/Engine.AnimSequenceBase|GetSequenceLength (Variables|Default|GetBlockAnim))))
    (Variables|Default|SetisBlocking false)))

(event EventAttemptHit
  (params (AttackingActor :type Actor%20Object%20Reference) (AttackDirection :type Vector :default "0, 0, 0") (AttackDamage :type Integer))
  ;[0.15 0.15 0.15 0.5] AttemptHit
  (Variables|Default|SetReceivedAttackDirection AttackDirection)
  (Variables|Default|SetReceivedAttackDamage AttackDamage)
  (if (< (Math|Vector|DotProduct (Transformation|GetActorForwardVector) (Math|Vector|Normalize (- (Transformation|GetActorLocation AttackingActor) (Transformation|GetActorLocation)))) 0.0) ; True : Attacking Actor is behind\nFalse : Attacking Actor is in front
    (CallFunction|ReceiveDamage (Variables|Default|GetReceivedAttackDamage) :!label _label)
    (elif (Variables|Default|GetisBlocking)
      (Utilities|FlowControl|Sequence
        (:then_0
          ;;[0.15 0.15 0.15 0.5] Reverse Left/Right Attack Direction
          (if (Utilities|Operators|EqualEqual (Variables|Default|GetReceivedAttackDirection) (Class|KismetMathLibrary|VectorRight) 0.0)
            (Variables|Default|SetReceivedAttackDirection (Class|KismetMathLibrary|VectorLeft))
            (elif (Utilities|Operators|EqualEqual (Variables|Default|GetReceivedAttackDirection) (Class|KismetMathLibrary|VectorLeft) 0.0)
              (Variables|Default|SetReceivedAttackDirection (Class|KismetMathLibrary|VectorRight)))))
        (:then_1
          ;;[0.15 0.15 0.15 0.5] Check if Strike is blocked
          (if (Utilities|Operators|EqualEqual (Variables|Default|GetActionDirection) (Variables|Default|GetReceivedAttackDirection) 0.0)
            (CallFunction|OnBlock)
            (else
              (CallFunction|ReceiveDamage (Variables|Default|GetReceivedAttackDamage))))))
      (else
        (goto _label)))))

(event EventDamage
  (params (AttackDamage :type Integer))
  ;[0.15 0.15 0.15 0.5] ReceiveDamage
  (Variables|Default|SetHealth (- (Variables|Default|GetHealth) AttackDamage))
  (bind _returnvalue (UserInterface|CreateWidget "/Game/GameAssets/Blueprints/Player/UI/WBP_RedBlur.WBP_RedBlur_C"))
  (UserInterface|Viewport|AddtoViewport _returnvalue 0)
  (Audio|PlaySound2D "/Game/GameAssets/Assets/SFX/Characters/SC_PainGrunts.SC_PainGrunts" 1.0 1.0 0.0 0 0))

(event EventOnBlock
  ;[0.15 0.15 0.15 0.5] Block
  (bind _returnvalue (UserInterface|CreateWidget "/Game/GameAssets/Blueprints/Player/UI/WBP_YellowBlur.WBP_YellowBlur_C"))
  (UserInterface|Viewport|AddtoViewport _returnvalue 0)
  (Audio|PlaySound2D "/Game/GameAssets/Assets/SFX/Characters/Weapons/SW_SwordParry.SW_SwordParry" 1.0 1.0 0.0 0 0))

(fn ConstructionScript)

(fn UpdateSpeedandFOV
  (if (Variables|Default|GetisSprinting)
    (Variables|Default|SetTargetFOV 1.2e+02)
    (Variables|Default|SetTargetSpeed 1e+03)
    (else
      (Variables|Default|SetTargetFOV 1.1e+02)
      (Variables|Default|SetTargetSpeed 5e+02))))

(fn GoRagdoll
  (bind _mesh (Variables|Character|GetMesh))
  (Variables|/Script/Engine.CameraComponent|SetbUsePawnControlRotation (Variables|Default|GetCamera) false)
  (Pawn|Components|CharacterMovement|DisableMovement (Variables|Character|GetCharacterMovement))
  (Collision|SetCollisionEnabled (Variables|Collision|GetCapsuleComponent) "NoCollision")
  (Physics|SetSimulatePhysics _mesh true)
  (Collision|SetCollisionProfileName _mesh "Ragdoll" true :!class /Script/Engine.PrimitiveComponent)
  ;[0.15 0.15 0.15 0.5] Add random impulse to avoid ragdoll always in same direction
  (Physics|AddImpulse (Variables|Character|GetMesh) (* (Math|Random|RandomUnitVector) "1000.000000,1000.000000,1000.000000") "None" true))

(fn GetinGameMenu
  (Variables|Default|GetWBP_InGameMenu
    (:then
      _)
    (:else
      (bind _returnvalue (UserInterface|CreateWidget "/CLM_MenuSystem/UI/Widgets/WBP_InGameMenu.WBP_InGameMenu_C" (Game|GetPlayerController 0)))
      (bind _output_get (Variables|Default|SetWBP_InGameMenu _returnvalue))))
  (return _output_get))

(fn SetSwordSocketsPosition
  (for (_array_element _array_index) (Variables|Default|GetSwordSockets)
    (Utilities|Array|SetArrayElem (Variables|Default|GetSwordOldSocketsPositions) _array_index (Transformation|GetSocketLocation (Variables|Default|GetSM_Sword_001_01) _array_element) true)))

(fn AttachBloodParticlestoBone
  (params (HitActor :type Actor%20Object%20Reference) (HitRelativeLocation :type Vector) (HitNormal :type Vector) (HitBone :type Name))
  (LocalVariables|SetHitActorVar HitActor)
  (LocalVariables|SetHitRelativeLocationVar HitRelativeLocation)
  (LocalVariables|SetHitNormalVar HitNormal)
  (LocalVariables|SetHitBoneVar HitBone)
  (if (Transformation|DoesSocketExist (Actor|GetComponentbyClass (LocalVariables|GetHitActorVar) "/Script/Engine.SkeletalMeshComponent") (LocalVariables|GetHitBoneVar)) ; If HitBone exists True, else False
    (AddComponent|AddNiagaraComponent (LocalVariables|GetHitActorVar) false (Math|Transform|MakeTransform (- (Transformation|GetSocketLocation (Actor|GetComponentbyClass (LocalVariables|GetHitActorVar) "/Script/Engine.SkeletalMeshComponent") (LocalVariables|GetHitBoneVar)) (Transformation|GetActorLocation (LocalVariables|GetHitActorVar))) (Math|Rotator|MakeRotfromZ (LocalVariables|GetHitNormalVar))))
    (else
      (AddComponent|AddNiagaraComponent (LocalVariables|GetHitActorVar) false (Math|Transform|MakeTransform (- (LocalVariables|GetHitRelativeLocationVar) (Transformation|GetActorLocation (LocalVariables|GetHitActorVar))) (Math|Rotator|MakeRotfromZ (LocalVariables|GetHitNormalVar)))))))