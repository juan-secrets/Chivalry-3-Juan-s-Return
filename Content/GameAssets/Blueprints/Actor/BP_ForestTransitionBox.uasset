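; BP_ForestTransitionBox is a trigger box that asks the player to confirm before travelling to another level.
; Player overlap switches input to UI-only with a cursor and shows a lazily created, cached confirmation dialogue, rebinding its response dispatcher.
; Yes plays a black fade, then shows a loading screen with level name and background before opening the level after timed delays.
; No restores game-only input and hides the cursor.
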(event OnComponentBeginOverlap(Box)
  (params (OverlappedComponent :type Primitive%20Component%20Object%20Reference) (OtherActor :type Actor%20Object%20Reference) (OtherComp :type Primitive%20Component%20Object%20Reference) (OtherBodyIndex :type Integer) (bFromSweep :type Boolean) (SweepResult :type Hit%20Result%20Structure%20%28by%20ref%29))
  (bind _returnvalue (Game|Player|GetPlayerPawn 0))
  (bind _returnvalue_2 (CallFunction|GetDialogue))
  (bind _returnvalue_3 (Game|GetPlayerController 0))
  (Utilities|Casting|CastToBP_Player _returnvalue)
  ;[0.15 0.15 0.15 0.5] Forest trigger box
  (if (== OtherActor _returnvalue)
    (Input|SetInputModeUIOnly _returnvalue_3 0 "DoNotLock" true)
    (Variables|/Script/Engine.PlayerController|SetbShowMouseCursor _returnvalue_3 true)
    (Default|ShowDialogue _returnvalue_2 (Variables|Default|GetMessage))
    (EventDispatchers|UnbindallEventsfromInputDispatch _returnvalue_2)
    (EventDispatchers|BindEventtoInputDispatch _returnvalue_2 (delegate Custom|OnLeaveConfirmation))))

(event Custom|OnLeaveConfirmation
  (params (Yes/No :type Boolean))
  (bind _returnvalue (Game|GetPlayerController 0))
  ;[0.15 0.15 0.15 0.5] Forest trigger box
  (if Yes/No
    (CallFunction|BlackFadein)
    (Utilities|FlowControl|Delay 1.0)
    (Widget|RemovefromParent (CallFunction|GetDialogue))
    (CallFunction|LoadingScene (Variables|Default|GetLevel%20Name) (Variables|Default|GetBackground))
    (Utilities|FlowControl|Delay 3.0)
    (Game|OpenLevel(byName) (Variables|Default|GetLevel))
    (Input|SetInputModeGameOnly _returnvalue false)
    (Variables|/Script/Engine.PlayerController|SetbShowMouseCursor _returnvalue false)
    (else
      (Input|SetInputModeGameOnly _returnvalue false)
      (Variables|/Script/Engine.PlayerController|SetbShowMouseCursor _returnvalue false))))

(fn ConstructionScript)

(fn GetDialogue
  (Variables|Default|GetWBP_ConfirmationDialogue
    (:then
      _)
    (:else
      (bind _returnvalue (UserInterface|CreateWidget "/CLM_MenuSystem/UI/Widgets/WBP_ConfirmationDialogue.WBP_ConfirmationDialogue_C" (Game|GetPlayerController 0)))
      (bind _output_get (Variables|Default|SetWBP_ConfirmationDialogue _returnvalue))))
  (return _output_get))

(fn LoadingScene
  (params (LevelName :type Text) (Background :type Texture%202D%20Object%20Reference))
  (Viewport|RemoveAllWidgets)
  (bind _returnvalue (UserInterface|CreateWidget "/CLM_MenuSystem/UI/Widgets/WBP_LoadingScreen.WBP_LoadingScreen_C" (Game|GetPlayerController 0) LevelName Background))
  (UserInterface|Viewport|AddtoViewport _returnvalue 0))

(fn BlackFadein
  (bind _returnvalue (UserInterface|CreateWidget "/CLM_MenuSystem/UI/Widgets/SubWidgets/WBP_BlackFadeIn.WBP_BlackFadeIn_C"))
  (UserInterface|Viewport|AddtoViewport _returnvalue 0)
  (UserInterface|Animation|PlayAnimation _returnvalue (Variables|/CLM_MenuSystem/UI/Widgets/SubWidgets/WBP_BlackFadeIn.WBP_BlackFadeIn_C|GetFadeIn _returnvalue) 0.0 1 "Forward" 1.0 false))