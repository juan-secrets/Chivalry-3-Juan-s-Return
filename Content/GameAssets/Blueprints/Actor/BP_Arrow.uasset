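; BP_Arrow is an arrow hazard that plays a whoosh near the player and sends hits to actors it touches.
; The WooshRadius overlap plays the sound only once, when BP_Player enters.
; Mesh overlap sends AttemptHit to the other actor through an interface message, with fixed damage and no direction.
; When the arrow itself receives AttemptHit, it sends that damage back to the attacking actor via ReceiveDamage.
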(event OnComponentBeginOverlap(WooshRadius)
  (params (OverlappedComponent :type Primitive%20Component%20Object%20Reference) (OtherActor :type Actor%20Object%20Reference) (OtherComp :type Primitive%20Component%20Object%20Reference) (OtherBodyIndex :type Integer) (bFromSweep :type Boolean) (SweepResult :type Hit%20Result%20Structure%20%28by%20ref%29))
  ;[0.15 0.15 0.15 0.5] Play woosh sound when close
  (Utilities|Casting|CastToBP_Player OtherActor)
  (if (not (Variables|Default|GetWooshPlayed))
    (Variables|Default|SetWooshPlayed true)
    (Audio|PlaySoundatLocation "/Game/GameAssets/Assets/SFX/arrow-whoosh.arrow-whoosh" (Transformation|GetActorLocation self) "0, 0, 0" 1.0 1.0 0.0 0 0 0 0)))

(event OnComponentBeginOverlap(StaticMesh)
  (params (OverlappedComponent :type Primitive%20Component%20Object%20Reference) (OtherActor :type Actor%20Object%20Reference) (OtherComp :type Primitive%20Component%20Object%20Reference) (OtherBodyIndex :type Integer) (bFromSweep :type Boolean) (SweepResult :type Hit%20Result%20Structure%20%28by%20ref%29))
  ;[0.15 0.15 0.15 0.5] Arrow hit
  (Class|BPIFighters|AttemptHit(Message) OtherActor self "0, 0, 0" 5))

(event EventAttemptHit
  (params (AttackingActor :type Actor%20Object%20Reference) (AttackDirection :type Vector :default "0, 0, 0") (AttackDamage :type Integer))
  ;[0.15 0.15 0.15 0.5] Arrow deals damage
  (Class|BPIFighters|ReceiveDamage(Message) AttackingActor AttackDamage))

(fn ConstructionScript)