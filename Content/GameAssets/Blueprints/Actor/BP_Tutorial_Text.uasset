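; BP_Tutorial_Text is a tutorial trigger actor that shows a dialog box while the player pawn stands inside its TriggerBox.
; On begin overlap it creates a WB_Dialog widget once, reuses it afterwards, adds it to the viewport and sets its text from the Dialogs array entry at TutoIndex.
; On end overlap by the player pawn it removes the widget from the viewport.
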(event OnComponentBeginOverlap(TriggerBox)
  (params (OverlappedComponent :type Primitive%20Component%20Object%20Reference) (OtherActor :type Actor%20Object%20Reference) (OtherComp :type Primitive%20Component%20Object%20Reference) (OtherBodyIndex :type Integer) (bFromSweep :type Boolean) (SweepResult :type Hit%20Result%20Structure%20%28by%20ref%29))
  ;[0.15 0.15 0.15 0.5] Display Tutorial dialgog box
  (if (== OtherActor (Game|Player|GetPlayerPawn 0))
    (Variables|Default|GetWBP_Dialog
      (:then
        (UserInterface|Viewport|AddtoViewport (Variables|Default|GetWBP_Dialog) 0))
      (:else
        (bind _returnvalue (UserInterface|CreateWidget "/Game/GameAssets/Blueprints/Dialogs/WB_Dialog.WB_Dialog_C" (Game|GetPlayerController 0)))
        (bind _output_get (Variables|Default|SetWBP_Dialog _returnvalue))
        (UserInterface|Viewport|AddtoViewport _output_get 0)))
    (Rendering|Components|TextRender|SetText (Variables|/Game/GameAssets/Blueprints/Dialogs/WB_Dialog.WB_Dialog_C|GetDialogText (Variables|Default|GetWBP_Dialog)) (Utilities|Text|ToText(String) (Utilities|Array|Get(acopy) (Variables|Default|GetDialogs) (Variables|Default|GetTutoIndex))))))

(event OnComponentEndOverlap(TriggerBox)
  (params (OverlappedComponent :type Primitive%20Component%20Object%20Reference) (OtherActor :type Actor%20Object%20Reference) (OtherComp :type Primitive%20Component%20Object%20Reference) (OtherBodyIndex :type Integer))
  ;[0.15 0.15 0.15 0.5] Remove Tuto from viewport
  (if (== OtherActor (Game|Player|GetPlayerPawn 0))
    (Widget|RemovefromParent (Variables|Default|GetWBP_Dialog))))

(fn ConstructionScript)