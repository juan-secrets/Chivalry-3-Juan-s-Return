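; Ranged enemy AI character that plays a bow montage, then fires an arrow at the player's upper spine, with a sword-overlap hit also wired.
; Incoming hits call for damage, report to AI perception and attach Niagara blood at the closest body collision point.
; Tick watches health to trigger death sounds and ragdoll, and bosses advance the player's progression index once.
; Helper functions supply ideal ranges, patrol route and walk speed.
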(event OnComponentBeginOverlap(SM_Sword_001_01)
  (params (OverlappedComponent :type Primitive%20Component%20Object%20Reference) (OtherActor :type Actor%20Object%20Reference) (OtherComp :type Primitive%20Component%20Object%20Reference) (OtherBodyIndex :type Integer) (bFromSweep :type Boolean) (SweepResult :type Hit%20Result%20Structure%20%28by%20ref%29))
  ;[0.15 0.15 0.15 0.5] Hit Player
  (if (and (Class|KismetMathLibrary|XORBoolean (Variables|Default|GetIs%20Attacking) (Variables|Default|GetAttack%20Input)) (!= OtherActor self))
    (Class|BPIFighters|AttemptHit(Message) OtherActor self (Variables|Default|GetAttackDirection) "0, 0, 0" 15)))

(event Custom|Fire%20Arrow
  (params (TargetActor :type Actor%20Object%20Reference))
  (bind _target (Variables|Default|GetTarget))
  (bind _arrowspawnpoint (Variables|Default|GetArrowSpawnPoint))
  (bind _returnvalue (Transformation|GetWorldLocation _arrowspawnpoint))
  (bind _mesh (Variables|/Script/Engine.Character|GetMesh _target))
  (bind _returnvalue_2 (Transformation|GetSocketLocation _mesh "spine_05"))
  (bind _returnvalue_3 (- _returnvalue_2 _returnvalue))
  (bind _returnvalue_4 (Math|Vector|Normalize _returnvalue_3))
  (bind _returnvalue_5 (Math|Rotator|MakeRotfromX _returnvalue_4))
  ;[0.15 0.15 0.15 0.5] Fire Arrow
  (bind _returnvalue_6 (Game|SpawnActorfromClass "/Game/GameAssets/Blueprints/Actor/BP_Arrow.BP_Arrow_C" (Math|Transform|MakeTransform (Transformation|GetWorldLocation (Variables|Default|GetArrowSpawnPoint)) _returnvalue_5 "1.000000,1.000000,1.000000") "Undefined" "MultiplyWithRoot" 0 0))
  (bind _output_get (Variables|Default|SetSpawnedArrow _returnvalue_6))
  (Variables|/Script/Engine.MovementComponent|SetVelocity (Variables|/Game/GameAssets/Blueprints/Actor/BP_Arrow.BP_Arrow_C|GetProjectileMovement _output_get) (* (Math|Vector|GetForwardVector _returnvalue_5) 2e+03)))

(event Custom|StopAttacking
  ;[0.15 0.15 0.15 0.5] Stop attacking
  (Variables|Default|SetAttack%20Input false)
  (Utilities|FlowControl|Delay 1.0)
  (Variables|Default|SetIs%20Attacking false))

(event EventDamage
  (params (AttackDamage :type Integer))
  ;[0.15 0.15 0.15 0.5] Set health
  (bind _output_get (Variables|Default|SetHealth (- (Variables|Default|GetHealth) AttackDamage)))
  (if (> _output_get 0)
    (Audio|PlaySound2D "/Game/GameAssets/Assets/SFX/Characters/Voices/NPC/SC_NPC_PainGrunts.SC_NPC_PainGrunts" 1.0 1.0 0.0 0 0)))

(event EventDeathRagdoll
  (bind _mesh (Variables|Character|GetMesh))
  ;[0.15 0.15 0.15 0.5] Death Ragdoll
  (Pawn|Components|CharacterMovement|DisableMovement (Variables|Character|GetCharacterMovement))
  (Collision|SetCollisionEnabled (Variables|Collision|GetCapsuleComponent) "NoCollision")
  (Physics|SetSimulatePhysics _mesh true)
  (Collision|SetCollisionProfileName _mesh "Ragdoll" true :!class /Script/Engine.PrimitiveComponent))

(event EventTick
  (params (DeltaSeconds :type Float%20%28single-precision%29))
  ;[0.15 0.15 0.15 0.5] Death and progression
  (if (<= (Variables|Default|GetHealth) 0)
    (if (Variables|Default|GetisDead)
      _
      (else
        (Variables|Default|SetisDead true)
        ;;[0.15 0.15 0.15 0.5] Play Death Sounds
        (Audio|PlaySound2D "/Game/GameAssets/Assets/SFX/Characters/Voices/NPC/NPC_DeathGrunt.NPC_DeathGrunt" 1.0 1.0 0.0 0 0)
        (Audio|PlaySound2D "/Game/GameAssets/Assets/SFX/Characters/SW_BodyFallImpact.SW_BodyFallImpact" 1.0 1.0 0.0 0 0 false)))
    (CallFunction|DeathRagdoll)
    (if (Variables|Default|GetIsBoss)
      (if (not (Variables|Default|GetProgressed))
        (bind _asbp_player (Utilities|Casting|CastToBP_Player (Game|Player|GetPlayerPawn 0)))
        (Variables|/Game/GameAssets/Blueprints/Player/BP_Player.BP_Player_C|SetProgressionIndex _asbp_player (+ (Variables|/Game/GameAssets/Blueprints/Player/BP_Player.BP_Player_C|GetProgressionIndex _asbp_player) 1))
        (Variables|Default|SetProgressed true)))))

(event EventAttack
  (params (TargetActor :type Actor%20Object%20Reference))
  ;[0.15 0.15 0.15 0.5] Ranged attack
  (bind _asbp_player (Utilities|Casting|CastToBP_Player TargetActor))
  (Variables|Default|SetTarget _asbp_player)
  (Variables|Default|SetAttack%20Input true)
  (if (not (Variables|Default|GetIs%20Attacking))
    (Variables|Default|SetIs%20Attacking true)
    (Audio|PlaySoundatLocation "/Game/GameAssets/Assets/SFX/Characters/Weapons/Bow/Bow_string.Bow_string" (Transformation|GetActorLocation self) "0, 0, 0" 1.0 1.0 0.0 "/Game/GameAssets/Assets/SFX/Characters/Weapons/Bow/SA_BowString.SA_BowString" 0 0 0)
    (Animation|Montage|PlayMontage (Variables|Character|GetMesh) "/Game/GameAssets/Assets/Animations/Bow/AM_BowAttack.AM_BowAttack"
      (:OnCompleted
        (CallFunction|FireArrow _asbp_player)
        (CallFunction|StopAttacking)))))

(event EventAttemptHit
  (params (AttackingActor :type Actor%20Object%20Reference) (AttackDirection :type Vector :default "0, 0, 0") (AttackLocation :type Vector :default "0, 0, 0") (AttackDamage :type Integer))
  ;[0.15 0.15 0.15 0.5] Taking damage
  (Variables|Default|SetReceivedAttackDirection AttackDirection)
  (bind _output_get (Variables|Default|SetReceivedAttackDamage AttackDamage))
  (if (< (Math|Vector|DotProduct (Transformation|GetActorForwardVector) (Math|Vector|Normalize (- (Transformation|GetActorLocation AttackingActor) (Transformation|GetActorLocation)))) 0.0)
    _
    (else
      _))
  (CallFunction|ReceiveDamage _output_get)
  (CallFunction|AttachBloodParticlestoActor self AttackLocation)
  ;[0.15 0.15 0.15 0.5] Damage perception
  (Class|AISenseDamage|ReportDamageEvent self (Game|Player|GetPlayerPawn 0) 0.0 "0, 0, 0" "0, 0, 0" "None"))

(fn ConstructionScript)

(fn AttachBloodParticlestoActor
  (params (HitActor :type Actor%20Object%20Reference) (HitLocation :type Vector))
  (LocalVariables|SetHitActorVar HitActor)
  (LocalVariables|SetHitLocationVar HitLocation)
  (for _array_element (Transformation|GetAllSocketNames (Actor|GetComponentbyClass (LocalVariables|GetHitActorVar) "/Script/Engine.SkeletalMeshComponent"))
    (if (> (.ReturnValue (Collision|GetClosestPointonCollision (Actor|GetComponentbyClass (LocalVariables|GetHitActorVar) "/Script/Engine.SkeletalMeshComponent") (LocalVariables|GetHitLocationVar) _array_element)) 0.0) ; Necessary because >= 0 is a fail to\nget the closest point
      (if (< (Math|Vector|VectorLength (- (.OutPointOnBody (Collision|GetClosestPointonCollision (Actor|GetComponentbyClass (LocalVariables|GetHitActorVar) "/Script/Engine.SkeletalMeshComponent") (LocalVariables|GetHitLocationVar) _array_element)) (LocalVariables|GetHitLocationVar))) (Math|Vector|VectorLength (- (LocalVariables|GetTempClosestLocation) (LocalVariables|GetHitLocationVar))))
        (LocalVariables|SetTempClosestLocation (.OutPointOnBody (Collision|GetClosestPointonCollision (Actor|GetComponentbyClass (LocalVariables|GetHitActorVar) "/Script/Engine.SkeletalMeshComponent") (LocalVariables|GetHitLocationVar) _array_element))))))
  (AddComponent|AddNiagaraComponent (LocalVariables|GetHitActorVar) false (Math|Transform|MakeTransform (- (LocalVariables|GetTempClosestLocation) (Transformation|GetActorLocation (LocalVariables|GetHitActorVar)))))
  (LocalVariables|SetTempClosestLocation "9999.000000,9999.000000,9999.000000"))

(fn GetIdealRange
  (return 1e+02 3.5e+02))

(fn GetPatrolRoute
  (return (Variables|AI|GetPatrolRoute)))

(fn SetMovementSpeed
  (params (Speed :type E_Movement_speed%20Enum :default "NewEnumerator0"))
  (bind _output_get (Variables|/Script/Engine.CharacterMovementComponent|SetMaxWalkSpeed (Variables|Character|GetCharacterMovement) (Utilities|Select :Index Speed :NewEnumerator0 0.0 :NewEnumerator1 1e+02 :NewEnumerator2 3e+02 :NewEnumerator3 5e+02)))
  (return _output_get))