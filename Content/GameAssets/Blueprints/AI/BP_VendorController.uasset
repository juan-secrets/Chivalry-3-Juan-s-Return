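; AI controller for a vendor NPC that wanders the level and stops to face the player during dialog.
; Movement alternates between random navigable points and random BP_waypoint actors gathered at BeginPlay, chained through delays and gated by IsInDialog.
; DialogStart halts movement and turns the pawn toward the player with a timeline-driven rotation lerp.
; DialogEnd only clears the flag; this graph neither starts nor resumes roaming itself.
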(event Custom|Start%20roaming
  ;[0.15 0.15 0.15 0.5] Roaming logic
  (if (not (Variables|Default|GetIsInDialog))
    (bind _randomlocation (Class|NavigationSystemV1|GetRandomLocationinNavigableRadius (Transformation|GetActorLocation (Pawn|GetControlledPawn)) (Variables|Default|GetRoamRadius) 0 0))
    (AI|AIMoveTo 0 _randomlocation 0 -1.0 "Default" "Default" true true
      (:then
        (if (Math|Random|RandomBool)
          (Utilities|FlowControl|Delay 1.0)
          (CallFunction|StartRoaming)
          (else
            (Utilities|FlowControl|Delay 2.5)
            (CallFunction|WaypointMovement)))))))

(event Custom|Waypoint%20movement
  ;[0.15 0.15 0.15 0.5] Waypoint movement
  (if (not (Variables|Default|GetIsInDialog))
    (AI|AIMoveTo (Pawn|GetControlledPawn) "0, 0, 0" (Utilities|Array|Get(acopy) (Variables|Default|GetWaypoint) (Math|Random|RandomIntegerinRange 0 (- (Utilities|Array|Length (Variables|Default|GetWaypoint)) 1))) 5e+02 false
      (:OnSuccess
        (Utilities|FlowControl|Delay 2.0)
        (CallFunction|StartRoaming))
      (:OnFail
        (CallFunction|WaypointMovement)))))

(event Custom|Dialog%20Start
  (params (PlayerRef :type BP%20Player%20Object%20Reference))
  (bind _returnvalue (Pawn|GetControlledPawn))
  ;[0.15 0.15 0.15 0.5] Look at player for dialog
  (Variables|Default|SetIsInDialog true)
  (AI|Navigation|StopMovement (Pawn|GetController _returnvalue))
  (Components|Timeline|PlayfromStart (Variables|Default|GetSmoothDialogLook))
  (bind _alpha (Timeline|SmoothDialogLook Play)
    (:Update
      (Transformation|SetActorRotation (Pawn|GetControlledPawn) (Math|Rotator|Lerp(Rotator) (Transformation|GetActorRotation _returnvalue) (Math|Rotator|FindLookatRotation (Transformation|GetActorLocation _returnvalue) (Transformation|GetActorLocation PlayerRef)) _alpha true)))))

(event Custom|Dialog%20End
  ;[0.15 0.15 0.15 0.5] Dialog End resume roaming
  (Variables|Default|SetIsInDialog false))

(event EventBeginPlay
  ;[0.15 0.15 0.15 0.5] Get all waypoints
  (bind _outactors (Actor|GetAllActorsOfClass "/Game/GameAssets/Blueprints/Actor/BP_waypoint.BP_waypoint_C"))
  (Variables|Default|SetWaypoint _outactors))

(fn ConstructionScript)