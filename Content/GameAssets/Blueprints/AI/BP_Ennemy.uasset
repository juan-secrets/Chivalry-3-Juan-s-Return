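; Sword-fighting enemy character that attacks endlessly from BeginPlay in random left, right, up or down directions.
; Each attack sets charge and slash montages, then times its phases with delays.
; Sword overlaps during the release phase send directional hit messages.
; Incoming hits apply damage without blocking (the facing check is empty), and Tick triggers a randomly impulsed ragdoll every frame while health is depleted.
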(event OnComponentBeginOverlap(SM_Sword_001_01)
  (params (OverlappedComponent :type Primitive%20Component%20Object%20Reference) (OtherActor :type Actor%20Object%20Reference) (OtherComp :type Primitive%20Component%20Object%20Reference) (OtherBodyIndex :type Integer) (bFromSweep :type Boolean) (SweepResult :type Hit%20Result%20Structure%20%28by%20ref%29))
  ;[0.15 0.15 0.15 0.5] Hit Player
  (if (and (Class|KismetMathLibrary|XORBoolean (Variables|Default|GetIs%20Attacking) (Variables|Default|GetAttack%20Input)) (!= OtherActor self))
    (Class|BPIFighters|AttemptHit(Message) OtherActor self (Variables|Default|GetAttackDirection) 15)))

(event Custom|Attack
  (Variables|Default|SetAttack%20Input true)
  (if (not (Variables|Default|GetIs%20Attacking))
    (switch int (Math|Random|RandomIntegerinRange 0 3)
      (:Default
        (Variables|Default|SetSwordChargeAnim "/Game/GameAssets/Assets/Animations/Sword/Charge/AM_L_SwordCharge.AM_L_SwordCharge" :!label _label)
        (Variables|Default|SetSwordSlashAnim "/Game/GameAssets/Assets/Animations/Sword/Slash/AM_L_SwordSlash.AM_L_SwordSlash")
        (Variables|Default|SetAttackDirection (Class|KismetMathLibrary|VectorLeft)))
      (:0
        (Variables|Default|SetSwordChargeAnim "/Game/GameAssets/Assets/Animations/Sword/Charge/AM_R_SwordCharge.AM_R_SwordCharge")
        (Variables|Default|SetSwordSlashAnim "/Game/GameAssets/Assets/Animations/Sword/Slash/AM_R_SwordSlash.AM_R_SwordSlash")
        (Variables|Default|SetAttackDirection (Class|KismetMathLibrary|VectorRight)))
      (:1
        (goto _label))
      (:2
        (Variables|Default|SetSwordChargeAnim "/Game/GameAssets/Assets/Animations/Sword/Charge/AM_T_SwordCharge.AM_T_SwordCharge")
        (Variables|Default|SetSwordSlashAnim "/Game/GameAssets/Assets/Animations/Sword/Slash/AM_T_SwordSlash.AM_T_SwordSlash")
        (Variables|Default|SetAttackDirection (Math|Vector|VectorUp)))
      (:3
        (Variables|Default|SetSwordChargeAnim "/Game/GameAssets/Assets/Animations/Sword/Charge/AM_B_SwordCharge.AM_B_SwordCharge")
        (Variables|Default|SetSwordSlashAnim "/Game/GameAssets/Assets/Animations/Sword/Slash/AM_B_SwordSlash.AM_B_SwordSlash")
        (Variables|Default|SetAttackDirection (Math|Vector|VectorDown))))
    (Variables|Default|SetIs%20Attacking true)
    (Utilities|FlowControl|Delay (Variables|Default|GetAttackChargeTime))
    (CallFunction|StopAttacking)))

(event Custom|StopAttacking
  (bind _swordchargeanim (Variables|Default|GetSwordChargeAnim))
  (bind _sequencelength (Variables|/Script/Engine.AnimSequenceBase|GetSequenceLength _swordchargeanim))
  (Variables|Default|SetAttack%20Input false)
  (Utilities|FlowControl|Delay (+ (Math|Float|Clamp(Float) (- _sequencelength (Variables|Default|GetAttackChargeTime)) 0.0 _sequencelength) (Variables|/Script/Engine.AnimSequenceBase|GetSequenceLength (Variables|Default|GetSwordSlashAnim))))
  (Variables|Default|SetIs%20Attacking false)
  (CallFunction|Attack))

(event EventDamage
  (params (AttackDamage :type Integer))
  ;[0.15 0.15 0.15 0.5] Take Damage
  (Variables|Default|SetHealth (- (Variables|Default|GetHealth) AttackDamage)))

(event EventBeginPlay
  (CallFunction|Attack))

(event EventAttemptHit
  (params (AttackingActor :type Actor%20Object%20Reference) (AttackDirection :type Vector :default "0, 0, 0") (AttackDamage :type Integer))
  (Variables|Default|SetReceivedAttackDirection AttackDirection)
  (bind _output_get (Variables|Default|SetReceivedAttackDamage AttackDamage))
  (if (< (Math|Vector|DotProduct (Transformation|GetActorForwardVector) (Math|Vector|Normalize (- (Transformation|GetActorLocation AttackingActor) (Transformation|GetActorLocation)))) 0.0)
    _
    (else
      _))
  (CallFunction|ReceiveDamage _output_get)
  (Development|PrintString "Aie je suis l'ennemi j'ai mal"))

(event EventTick
  (params (DeltaSeconds :type Float%20%28single-precision%29))
  (if (<= (Variables|Default|GetHealth) 0)
    (CallFunction|DeathRagdoll)))

(fn ConstructionScript)

(fn DeathRagdoll
  (bind _mesh (Variables|Character|GetMesh))
  (Pawn|Components|CharacterMovement|DisableMovement (Variables|Character|GetCharacterMovement))
  (Collision|SetCollisionEnabled (Variables|Collision|GetCapsuleComponent) "NoCollision")
  (Physics|SetSimulatePhysics _mesh true)
  (Collision|SetCollisionProfileName _mesh "Ragdoll" true :!class /Script/Engine.PrimitiveComponent)
  ;[0.15 0.15 0.15 0.5] Add random impulse to avoid ragdoll always in same direction
  (Physics|AddImpulse (Variables|Character|GetMesh) (* (Math|Random|RandomUnitVector) "1000.000000,1000.000000,1000.000000") "None" true))