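; Behavior tree node that locates the player around the AI-controlled pawn.
; On each AI tick it runs a multi sphere trace for Pawn objects at the pawn's location, with the radius read from the blackboard and debug drawing on.
; A BP_Player among the hits is written to the TargetActor blackboard key, which is cleared when none is found.
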(event EventReceiveTickAI
  (params (OwnerController :type AI%20Controller%20Object%20Reference) (ControlledPawn :type Pawn%20Object%20Reference) (DeltaSeconds :type Float%20%28single-precision%29))
  (bind _returnvalue (Transformation|GetActorLocation ControlledPawn))
  (bind _targetactor (Variables|Default|GetTargetActor))
  (Variables|Default|SetPlayerRef 0)
  (bind (_outhits _returnvalue_2) (Collision|MultiSphereTraceForObjects _returnvalue _returnvalue (Class|BTFunctionLibrary|GetBlackboardValueasFloat (Variables|Default|GetSearchRadius)) (Utilities|Array|MakeArray "ObjectTypeQuery3") false 0 "ForDuration"))
  (if _returnvalue_2
    (for _array_element _outhits
      (bind _asbp_player (Utilities|Casting|CastToBP_Player (.HitActor (Collision|BreakHitResult _array_element))))
      (Variables|Default|SetPlayerRef _asbp_player)))
  (Utilities|IsValid (Variables|Default|GetPlayerRef)
    (:Is%20Valid
      (Class|BTFunctionLibrary|SetBlackboardValueasObject _targetactor (Variables|Default|GetPlayerRef)))
    (:Is%20Not%20Valid
      (Class|BTFunctionLibrary|ClearBlackboardValue _targetactor))))