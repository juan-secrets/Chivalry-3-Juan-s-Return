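; Old man villager NPC that gives tutorial dialogue to the player.
; Its trigger box shows an input prompt widget while the player is inside and clears the prompt and any open dialogue on exit.
; Each OldManTalk call notifies the villager AI controller and shows the next Dialog line, closing and resetting after the last.
; Walking away leaves the line index intact, so the conversation resumes where it stopped.
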(event OnComponentBeginOverlap(TriggerBox)
  (params (OverlappedComponent :type Primitive%20Component%20Object%20Reference) (OtherActor :type Actor%20Object%20Reference) (OtherComp :type Primitive%20Component%20Object%20Reference) (OtherBodyIndex :type Integer) (bFromSweep :type Boolean) (SweepResult :type Hit%20Result%20Structure%20%28by%20ref%29))
  ;[0.15 0.15 0.15 0.5] Input display
  (if (== OtherActor (Variables|Default|GetAs%20BP%20Player))
    (Variables|Default|GetDialogInputUI
      (:then
        (UserInterface|Viewport|AddtoViewport (Variables|Default|GetDialogInputUI) 0))
      (:else
        (bind _returnvalue (UserInterface|CreateWidget "/Game/GameAssets/Blueprints/Dialogs/WB_Dialog_input.WB_Dialog_input_C" (Game|GetPlayerController 0)))
        (bind _output_get (Variables|Default|SetDialogInputUI _returnvalue))
        (UserInterface|Viewport|AddtoViewport _output_get 0)))))

(event OnComponentEndOverlap(TriggerBox)
  (params (OverlappedComponent :type Primitive%20Component%20Object%20Reference) (OtherActor :type Actor%20Object%20Reference) (OtherComp :type Primitive%20Component%20Object%20Reference) (OtherBodyIndex :type Integer))
  ;[0.15 0.15 0.15 0.5] Leave villager
  (if (== OtherActor (Variables|Default|GetAs%20BP%20Player))
    (bind _dialogui (Variables|Default|GetDialogUI)
      (:then
        (Widget|RemovefromParent _dialogui)
        (Variables|Default|SetDialogUI 0)
        (bind _dialoginputui (Variables|Default|GetDialogInputUI)
          (:then
            (Widget|RemovefromParent _dialoginputui)
            (Variables|Default|SetDialogInputUI 0)
            (Default|DialogEnd (Variables|Default|GetAs%20BP%20Villager%20Controller)))
          (:else)))
      (:else
        (bind _dialoginputui_2 (Variables|Default|GetDialogInputUI)
          (:then
            (Widget|RemovefromParent _dialoginputui_2)
            (Variables|Default|SetDialogInputUI 0))
          (:else))))))

(event EventBeginPlay
  ;[0.15 0.15 0.15 0.5] Set player and controller refs
  (bind _asbp_player (Utilities|Casting|CastToBP_Player (Game|GetPlayerCharacter 0)))
  (Variables|Default|SetAs%20BP%20Player _asbp_player)
  (bind _asbp_villager_controller (Utilities|Casting|CastToBP_Villager_controller (Pawn|GetController)))
  (Variables|Default|SetAs%20BP%20Villager%20Controller _asbp_villager_controller)
  (Variables|/Script/Engine.CharacterMovementComponent|SetMaxWalkSpeed (Variables|Character|GetCharacterMovement) (Variables|Default|GetTargetSpeed)))

(event EventOldManTalk
  ;[0.15 0.15 0.15 0.5] Tutorial Dialog
  (Default|DialogStart (Variables|Default|GetAs%20BP%20Villager%20Controller) (Variables|Default|GetAs%20BP%20Player))
  (Variables|Default|GetDialogUI
    (:then
      (UserInterface|Viewport|AddtoViewport (Variables|Default|GetDialogUI) 0))
    (:else
      (bind _returnvalue (UserInterface|CreateWidget "/Game/GameAssets/Blueprints/Dialogs/WB_Dialog.WB_Dialog_C" (Game|GetPlayerController 0)))
      (bind _output_get (Variables|Default|SetDialogUI _returnvalue))
      (UserInterface|Viewport|AddtoViewport _output_get 0)))
  (Rendering|Components|TextRender|SetText (Variables|/Game/GameAssets/Blueprints/Dialogs/WB_Dialog.WB_Dialog_C|GetDialogText (Variables|Default|GetDialogUI)) (Utilities|Text|ToText(String) (Utilities|Array|Get(acopy) (Variables|Default|GetDialog) (Variables|Default|GetTalkIndex))))
  (if (< (Variables|Default|GetTalkIndex) (Utilities|Array|Length (Variables|Default|GetDialog)))
    (Math|Integer|IncrementInt (Variables|Default|GetTalkIndex))
    (else
      (Widget|RemovefromParent (Variables|Default|GetDialogUI))
      (Variables|Default|SetTalkIndex 0)
      (Variables|Default|SetDialogUI 0)
      (Default|DialogEnd (Variables|Default|GetAs%20BP%20Villager%20Controller)))))

(fn ConstructionScript)