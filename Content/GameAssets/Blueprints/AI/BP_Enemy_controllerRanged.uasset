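; AI controller for ranged enemies that runs BT_EnemyRanged and drives its Passive, Investigating, Attacking and Dead states.
; On possess it starts Passive and copies the pawn's attack and defend radii to the Blackboard.
; Perception updates are split by sense: seeing the player or taking damage triggers Attacking, while sounds trigger Investigating.
; These reactions apply only while Passive or Investigating, with state, target and point of interest written to the Blackboard.
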(event OnPerceptionUpdated(AIPerception)
  (params (UpdatedActors :type Array%20of%20Actor%20Object%20References))
  ;[0.15 0.15 0.15 0.5] Respond to Perception Stimuli Sight/Sound/Damage
  (for _array_element UpdatedActors
    (Utilities|FlowControl|Sequence
      (:then_0
        (bind _sensed (CallFunction|CanSenseActor _array_element "NewEnumerator1"))
        (if _sensed
          (CallFunction|HandleSensedSight _array_element)))
      (:then_1
        (bind (_sensed_2 _stimulus) (CallFunction|CanSenseActor _array_element "NewEnumerator2"))
        (if _sensed_2
          (CallFunction|HandleSensedSound (.StimulusLocation (Utilities|Struct|BreakAIStimulus _stimulus)))))
      (:then_2
        (bind _sensed_3 (CallFunction|CanSenseActor _array_element "NewEnumerator3"))
        (if _sensed_3
          (CallFunction|HandleSensedDamage _array_element))))))

(event EventPossess
  (params (PossessedPawn :type Pawn%20Object%20Reference))
  ;[0.15 0.15 0.15 0.5] Run behavior tree
  (Variables|Default|SetPossessed%20Pawn PossessedPawn)
  (AI|RunBehaviorTree "/Game/GameAssets/Blueprints/AI/Behavior/BT_EnemyRanged.BT_EnemyRanged")
  (CallFunction|SetStatePassive)
  (bind (_attackradius _defendradius) (Class|BPIEnemy|GetIdealRange(Message) PossessedPawn))
  (AI|Components|Blackboard|SetValueasFloat (Variables|Default|GetBlackboard) (Variables|Default|GetAttackRadiusKeyName) _attackradius)
  (AI|Components|Blackboard|SetValueasFloat (Variables|Default|GetBlackboard) (Variables|Default|GetDefendRadiusKeyName) _defendradius))

(fn ConstructionScript)

(fn SetStatePassive
  (AI|Components|Blackboard|SetValueasEnum (Variables|Default|GetBlackboard) (Variables|Default|GetStateKeyName) (Utilities|Enum|LiteralenumE_IA_State "NewEnumerator0")))

(fn SetStateAttacking
  (params (AttackTarget :type Actor%20Object%20Reference))
  (AI|Components|Blackboard|SetValueasObject (Variables|Default|GetBlackboard) (Variables|Default|GetTargetActorKeyName) AttackTarget)
  (AI|Components|Blackboard|SetValueasEnum (Variables|Default|GetBlackboard) (Variables|Default|GetStateKeyName) (Utilities|Enum|LiteralenumE_IA_State "NewEnumerator1"))
  (Variables|Default|SetAttack%20Target AttackTarget))

(fn CanSenseActor
  (params (Actor :type Actor%20Object%20Reference) (Sense :type E_AI_Senses%20Enum :default "NewEnumerator0"))
  (bind _info (Class|AIPerceptionComponent|GetActorsPerception (Variables|Default|GetAIPerception) Actor))
  (for _array_element (.LastSensedStimuli (Utilities|Struct|BreakActorPerceptionBlueprintInfo _info))
    (bind _returnvalue (Class|AIPerceptionSystem|GetSenseClassforStimulus _array_element))
    (if (== _returnvalue (Utilities|Select :Index Sense :NewEnumerator0 0 :NewEnumerator1 "/Script/AIModule.AISense_Sight" :NewEnumerator2 "/Script/AIModule.AISense_Hearing" :NewEnumerator3 "/Script/AIModule.AISense_Damage"))
      (return (.bSuccessfullySensed (Utilities|Struct|BreakAIStimulus _array_element)) _array_element))))

(fn HandleSensedSight
  (params (Actor :type Actor%20Object%20Reference))
  (bind _state (CallFunction|GetCurrentState))
  (switch Utilities|FlowControl|Switch|SwitchonE_IA_State _state
    (:NewEnumerator0
      _)
    (:NewEnumerator3
      _))
  (if (== Actor (Game|GetPlayerCharacter 0))
    (CallFunction|SetStateAttacking Actor)))

(fn GetCurrentState
  (return (Utilities|Enum|ByteToEnumE_IA_State (Class|BlackboardComponent|GetValueasEnum (Variables|Default|GetBlackboard) (Variables|Default|GetStateKeyName)))))

(fn HandleSensedSound
  (params (Location :type Vector))
  (bind _state (CallFunction|GetCurrentState))
  (switch Utilities|FlowControl|Switch|SwitchonE_IA_State _state
    (:NewEnumerator0
      _)
    (:NewEnumerator3
      _))
  (CallFunction|SetStateInvestigate Location))

(fn SetStateInvestigate
  (params (Location :type Vector))
  (AI|Components|Blackboard|SetValueasEnum (Variables|Default|GetBlackboard) (Variables|Default|GetStateKeyName) (Utilities|Enum|LiteralenumE_IA_State "NewEnumerator3"))
  (AI|Components|Blackboard|SetValueasVector (Variables|Default|GetBlackboard) (Variables|Default|GetPointOfInterestKeyName) Location))

(fn HandleSensedDamage
  (params (Actor :type Actor%20Object%20Reference))
  (bind _state (CallFunction|GetCurrentState))
  (switch Utilities|FlowControl|Switch|SwitchonE_IA_State _state
    (:NewEnumerator0
      _)
    (:NewEnumerator3
      _))
  (CallFunction|SetStateAttacking Actor))

(fn SetStateDead
  (AI|Components|Blackboard|SetValueasEnum (Variables|Default|GetBlackboard) (Variables|Default|GetStateKeyName) (Utilities|Enum|LiteralenumE_IA_State "NewEnumerator4")))