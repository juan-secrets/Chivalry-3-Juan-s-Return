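; Villager AI controller that makes its pawn wander around a village, alternating between waypoint travel and local roaming.
; On BeginPlay it gathers all BP_waypoint actors and moves to a random one, using a hardcoded index range that assumes ten waypoints.
; On arrival it waits, then roams to a random navigable point within RoamRadius before randomly roaming again or picking a new waypoint.
; Failed waypoint moves immediately retry with another random pick.
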(event Custom|Start%20roaming
  ;[0.15 0.15 0.15 0.5] Roaming logic
  (bind _randomlocation (Class|NavigationSystemV1|GetRandomLocationinNavigableRadius (Transformation|GetActorLocation (Pawn|GetControlledPawn)) (Variables|Default|GetRoamRadius) 0 0))
  (AI|AIMoveTo 0 _randomlocation 0 -1.0 "Default" "Default" true true
    (:then
      (if (Math|Random|RandomBool)
        (Utilities|FlowControl|Delay 1.0)
        (CallFunction|StartRoaming)
        (else
          (Utilities|FlowControl|Delay 2.5)
          (CallFunction|WaypointMovement))))))

(event Custom|Waypoint%20movement
  ;[0.15 0.15 0.15 0.5] Waypoint movement
  (AI|AIMoveTo (Pawn|GetControlledPawn) "0, 0, 0" (Utilities|Array|Get(acopy) (Variables|Default|GetWaypoint) (Math|Random|RandomIntegerinRange 0 9)) 5e+02 false
    (:OnSuccess
      (Utilities|FlowControl|Delay 2.0)
      (CallFunction|StartRoaming))
    (:OnFail
      (CallFunction|WaypointMovement))))

(event EventBeginPlay
  (bind _outactors (Actor|GetAllActorsOfClass "/Game/GameAssets/Blueprints/Actor/BP_waypoint.BP_waypoint_C"))
  (Variables|Default|SetWaypoint _outactors)
  (CallFunction|WaypointMovement))

(fn ConstructionScript)