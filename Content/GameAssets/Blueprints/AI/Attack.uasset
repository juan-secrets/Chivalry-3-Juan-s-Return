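; Behavior Tree task that makes an AI pawn attack its blackboard Target.
; On execute it sends AttackMessage to the pawn and finishes successfully at once, but never finishes if the Target is invalid.
; A separate Attackbase event, not called here, randomly picks one of four sword directions with matching charge and slash animations.
; It holds AttackInput for the charge time, then StopAttacking clears IsAttacking after a delay derived from animation lengths.
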(event Custom|Attackbase
  (Variables|Default|SetAttackInput true)
  (if (not (Variables|Default|GetIsAttacking))
    (switch int (Math|Random|RandomIntegerinRange 0 3)
      (:Default
        (Variables|Default|SetSwordChargeAnim "/Game/GameAssets/Assets/Animations/Sword/Charge/AM_L_SwordCharge.AM_L_SwordCharge" :!label _label)
        (Variables|Default|SetSwordSlashAnim "/Game/GameAssets/Assets/Animations/Sword/Slash/AM_L_SwordSlash.AM_L_SwordSlash")
        (Variables|Default|SetAttackDirection (Class|KismetMathLibrary|VectorLeft)))
      (:0
        (Variables|Default|SetSwordChargeAnim "/Game/GameAssets/Assets/Animations/Sword/Charge/AM_R_SwordCharge.AM_R_SwordCharge")
        (Variables|Default|SetSwordSlashAnim "/Game/GameAssets/Assets/Animations/Sword/Slash/AM_R_SwordSlash.AM_R_SwordSlash")
        (Variables|Default|SetAttackDirection (Class|KismetMathLibrary|VectorRight)))
      (:1
        (goto _label))
      (:2
        (Variables|Default|SetSwordChargeAnim "/Game/GameAssets/Assets/Animations/Sword/Charge/AM_T_SwordCharge.AM_T_SwordCharge")
        (Variables|Default|SetSwordSlashAnim "/Game/GameAssets/Assets/Animations/Sword/Slash/AM_T_SwordSlash.AM_T_SwordSlash")
        (Variables|Default|SetAttackDirection (Math|Vector|VectorUp)))
      (:3
        (Variables|Default|SetSwordChargeAnim "/Game/GameAssets/Assets/Animations/Sword/Charge/AM_B_SwordCharge.AM_B_SwordCharge")
        (Variables|Default|SetSwordSlashAnim "/Game/GameAssets/Assets/Animations/Sword/Slash/AM_B_SwordSlash.AM_B_SwordSlash")
        (Variables|Default|SetAttackDirection (Math|Vector|VectorDown))))
    (Variables|Default|SetIsAttacking true)
    (Utilities|FlowControl|Delay (Variables|Default|GetAttackChargeTime))
    (CallFunction|StopAttacking)))

(event Custom|StopAttacking
  (bind _swordchargeanim (Variables|Default|GetSwordChargeAnim))
  (bind _sequencelength (Variables|/Script/Engine.AnimSequenceBase|GetSequenceLength _swordchargeanim))
  (Variables|Default|SetAttackInput false)
  (Utilities|FlowControl|Delay (+ (Math|Float|Clamp(Float) (- _sequencelength (Variables|Default|GetAttackChargeTime)) 0.0 _sequencelength) (Variables|/Script/Engine.AnimSequenceBase|GetSequenceLength (Variables|Default|GetSwordSlashAnim))))
  (Variables|Default|SetIsAttacking false))

(event EventReceiveExecuteAI
  (params (OwnerController :type AI%20Controller%20Object%20Reference) (ControlledPawn :type Pawn%20Object%20Reference))
  (bind _target (Variables|Default|GetTarget))
  (bind _returnvalue (AI|BehaviorTree|GetBlackboardValueasActor _target))
  (Utilities|IsValid _returnvalue
    (:Is%20Valid
      (Class|BPIEnemy|Attack(Message) ControlledPawn _returnvalue)
      (AI|BehaviorTree|FinishExecute true))))